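; Bullet projectile actor that flies as a physics body and pushes the physics objects it hits.
; On BeginPlay, its Sphere component receives a large impulse along its forward vector to launch it.
; On Hit, if the other component simulates physics, it receives an impulse at the bullet's location, scaled from the bullet's current velocity.
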(event EventBeginPlay
  ;[1 1 1] 添加子弹初速度
  (Physics|AddImpulse (Variables|MyProjectile|GetSphere) (* (Math|Vector|GetForwardVector (Transformation|GetWorldRotation (Variables|MyProjectile|GetSphere))) 10000) "None" false))

(event Collision|EventHit
  (params (MyComp :type Primitive%20Component%20Object%20Reference) (Other :type Actor%20Object%20Reference) (OtherComp :type Primitive%20Component%20Object%20Reference) (bSelfMoved :type Boolean) (HitLocation :type Vector :default "0, 0, 0") (HitNormal :type Vector :default "0, 0, 0") (NormalImpulse :type Vector :default "0, 0, 0") (Hit :type Hit%20Result%20Structure%20%28by%20ref%29))
  ;[1 1 1] 击中物体后给物体添加冲量
  (if (Physics|IsSimulatingPhysics OtherComp "None")
    (Physics|AddImpulseatLocation OtherComp (* (Transformation|GetVelocity) 5e+02) (Transformation|GetActorLocation) "None")))

(fn ConstructionScript)